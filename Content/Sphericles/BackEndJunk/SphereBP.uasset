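; Sphericles sphere actor that slowly drifts downward and pops with a sound, destroying itself, when it overlaps the player pawn class SphericlesPawn2BP.
; Construction randomly applies one of two materials.
; Each Tick checks overlap before and after the swept move; a post-move overlap starts an attached tone, gated by CanPlay.
; Without overlap, a distant player stops the tone and re-arms CanPlay; the timer-based re-arm is unconnected.
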(event Custom|allowPlay
  (Variables|Default|SetcanPlay true))

(event EventBeginPlay)

(event EventTick
  (params (DeltaSeconds :type Float%20%28single-precision%29))
  (if (> (Utilities|Array|Length (Collision|GetOverlappingActors "/Game/Sphericles/BackEndJunk/SphericlesPawn2BP.SphericlesPawn2BP_C" :!class /Script/Engine.PrimitiveComponent)) 0)
    (Actor|DestroyActor)
    (Audio|PlaySoundatLocation "/Game/Sphericles/ToneCues/pop.pop" (Transformation|GetActorLocation))
    (else
      (Transformation|AddLocalOffset "0, 0,-0.008000" true)
      (if (> (Utilities|Array|Length (Collision|GetOverlappingActors "/Game/Sphericles/BackEndJunk/SphericlesPawn2BP.SphericlesPawn2BP_C" :!class /Script/Engine.PrimitiveComponent)) 0)
        (if (Variables|Default|GetcanPlay)
          (Variables|Default|SetcanPlay false)
          (bind _returnvalue (Class|GameplayStatics|PlaySoundAttached "/Game/Sphericles/ToneCues/DiTone.DiTone" (Variables|Default|GetSphere1) "None" (Transformation|GetActorLocation) "KeepWorldPosition" true)))
        (else
          (bind _returnvalue_2 (Transformation|GetDistanceTo (Game|Player|GetPlayerPawn 0)))
          (if (> _returnvalue_2 5e+03)
            (Audio|Components|Audio|Stop _returnvalue)
            (Variables|Default|SetcanPlay true)))))))

(fn ConstructionScript
  (if (Math|Random|RandomBool)
    (Rendering|Material|SetMaterial 0 "/Game/Sphericles/BackEndJunk/Sharp.Sharp")
    (else
      (Rendering|Material|SetMaterial (Variables|Default|GetStaticMesh1) 0 "/Game/Sphericles/BackEndJunk/TestMaterial.TestMaterial"))))