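; Sphericles pawn that flies continuously along its local forward axis and steers with click-and-drag mouse input.
; The MoveForward axis ramps Speed between MinSpeed and MaxSpeed, and Tick applies it as a swept local offset.
; While Click is held, mouse axes accumulate into values applied every tick as local yaw, then pitch, so drag distance sets turn rate.
; Releasing Click zeroes both values.
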(event EventTick
  (params (DeltaSeconds :type Float%20%28single-precision%29))
  (Transformation|AddActorLocalOffset (Math|Vector|MakeVector (* DeltaSeconds (Variables|Default|GetSpeed)) 0.0 0.0) true)
  (if (Variables|Default|GetmousePressed)
    (Variables|Default|SetPitchSet (* (Variables|Default|GetmouseYRec) 1.0))
    (Variables|Default|SetYawSet (* (Variables|Default|GetmouseXRec) 1.0))
    (Transformation|AddActorLocalRotation (Class|KismetMathLibrary|MakeRot 0.0 (Variables|Default|GetYawSet) 0.0) false)
    (Transformation|AddActorLocalRotation (Class|KismetMathLibrary|MakeRot (Variables|Default|GetPitchSet) 0.0 0.0) false)))

(event Input|ActionEvents|InputActionClick
  (:Pressed
    (Variables|Default|SetmousePressed true))
  (:Released
    (Variables|Default|SetmousePressed false)
    (Variables|Default|SetmouseXRec 0.0)
    (Variables|Default|SetmouseYRec 0.0)))

(event Input|AxisEvents|InputAxisLookUp
  (params (AxisValue :type Float%20%28single-precision%29))
  (Variables|Default|SetmouseYRec (+ (* AxisValue (Utilities|Time|GetWorldDeltaSeconds) (Math|Conversions|ToFloat(Boolean) (Variables|Default|GetmousePressed)) 1.0) (Variables|Default|GetmouseYRec))))

(event Input|AxisEvents|InputAxisMoveForward
  (params (AxisValue :type Float%20%28single-precision%29))
  (Variables|Default|SetSpeed (Math|Float|Clamp(Float) (+ (* AxisValue (Utilities|Time|GetWorldDeltaSeconds) (* (- (Variables|Default|GetMaxSpeed) (Variables|Default|GetMinSpeed)) 0.1)) (Variables|Default|GetSpeed)) (Variables|Default|GetMinSpeed) (Variables|Default|GetMaxSpeed))))

(event Input|AxisEvents|InputAxisLookRight
  (params (AxisValue :type Float%20%28single-precision%29))
  (Variables|Default|SetmouseXRec (+ (* AxisValue (Utilities|Time|GetWorldDeltaSeconds) (Math|Conversions|ToFloat(Boolean) (Variables|Default|GetmousePressed)) 1.0) (Variables|Default|GetmouseXRec))))

(fn ConstructionScript)