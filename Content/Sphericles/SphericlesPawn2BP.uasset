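; SphericlesPawn2BP is a player-controlled pawn that flies through the level with free look and movement on three input axes.
; Look input applies local pitch and world yaw scaled by TurnSpeed and frame time.
; MoveForward, MoveRight and MoveUp share one swept local offset scaled by Speed and frame time.
; EnableMovement sets StopMovingOnWall, which these graphs never read, and the hit and overlap events are empty.
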(event EventHit
  (params (MyComp :type Primitive%20Component%20Object%20Reference) (Other :type Actor%20Object%20Reference) (OtherComp :type Primitive%20Component%20Object%20Reference) (bSelfMoved :type Boolean) (HitLocation :type Vector :default "0, 0, 0") (HitNormal :type Vector :default "0, 0, 0") (NormalImpulse :type Vector :default "0, 0, 0") (Hit :type Hit%20Result%20Structure%20%28by%20ref%29)))

(event EventActorBeginOverlap
  (params (OtherActor :type Actor%20Object%20Reference)))

(event Input|AxisEvents|InputAxisLookUp
  (params (AxisValue :type Float%20%28single-precision%29))
  (Transformation|AddActorLocalRotation self (Class|KismetMathLibrary|MakeRot (* AxisValue (Utilities|Time|GetWorldDeltaSeconds) (Variables|Default|GetTurnSpeed)) 0.0 0.0) false))

(event Input|AxisEvents|InputAxisMoveUp
  (params (AxisValue :type Float%20%28single-precision%29))
  (Transformation|AddActorLocalOffset self (Math|Vector|MakeVector (* (stale Input|AxisEvents|InputAxisMoveForward AxisValue) (Utilities|Time|GetWorldDeltaSeconds) (Variables|Default|GetSpeed)) (* (stale Input|AxisEvents|InputAxisMoveRight AxisValue) (Utilities|Time|GetWorldDeltaSeconds) (Variables|Default|GetSpeed)) (* AxisValue (Utilities|Time|GetWorldDeltaSeconds) (Variables|Default|GetSpeed))) true))

(event Input|AxisEvents|InputAxisMoveForward
  (params (AxisValue :type Float%20%28single-precision%29))
  (Transformation|AddActorLocalOffset self (Math|Vector|MakeVector (* AxisValue (Utilities|Time|GetWorldDeltaSeconds) (Variables|Default|GetSpeed)) (* (stale Input|AxisEvents|InputAxisMoveRight AxisValue) (Utilities|Time|GetWorldDeltaSeconds) (Variables|Default|GetSpeed)) (* (stale Input|AxisEvents|InputAxisMoveUp AxisValue) (Utilities|Time|GetWorldDeltaSeconds) (Variables|Default|GetSpeed))) true))

(event Input|AxisEvents|InputAxisLookRight
  (params (AxisValue :type Float%20%28single-precision%29))
  (Class|Actor|AddActorWorldRotation self (Class|KismetMathLibrary|MakeRot 0.0 (* AxisValue (Utilities|Time|GetWorldDeltaSeconds) (Variables|Default|GetTurnSpeed)) 0.0)))

(event Input|AxisEvents|InputAxisMoveRight
  (params (AxisValue :type Float%20%28single-precision%29))
  (Transformation|AddActorLocalOffset self (Math|Vector|MakeVector (* (stale Input|AxisEvents|InputAxisMoveForward AxisValue) (Utilities|Time|GetWorldDeltaSeconds) (Variables|Default|GetSpeed)) (* AxisValue (Utilities|Time|GetWorldDeltaSeconds) (Variables|Default|GetSpeed)) (* (stale Input|AxisEvents|InputAxisMoveUp AxisValue) (Utilities|Time|GetWorldDeltaSeconds) (Variables|Default|GetSpeed))) true))

(fn ConstructionScript)

(fn EnableMovement
  (Variables|Default|SetStopMovingOnWall 1.0))